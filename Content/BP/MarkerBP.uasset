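; Marker visualiser that shows tracked marker positions and their true/false labels on a set of spheres.
; On BeginPlay it enables player input, then calls InitTracking and ReadFile.
; Each press of N fetches marker-label pairs from GetMarkerLabel, moves the sphere at each matching index to its marker position, and applies a right or wrong material according to the label.
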(event `self.ReceiveBeginPlay`
  (`self.EnableInput` (`GameplayStatics.GetPlayerController` 0))
  (`self.InitTracking`)
  (`self.ReadFile`))

(event `Key|N`
  (params (Key :type "Key Structure"))
  (:`Pressed`
    (`KismetSystemLibrary.PrintString` "Hello")
    (bind _returnvalue (`self.GetMarkerLabel`))
    (for (_array_element _array_index) _returnvalue
      (bind _output (`|GetArrayItem` (`self.Spheres`) _array_index))
      (bind (_marker _label) (break `MarkerLabel` _array_element))
      (`self.K2_SetActorLocation` _output _marker false false)
      (if _label
        (set `self.LabelMaterial` "/OptiTracking/Materials/M_RightLabel.M_RightLabel")
        (else
          (set `self.LabelMaterial` "/OptiTracking/Materials/M_WrongLabel.M_WrongLabel")))
      (`PrimitiveComponent.SetMaterial` (`StaticMeshActor.StaticMeshComponent` _output) 0 (`self.LabelMaterial`)))))

(fn `UserConstructionScript`)